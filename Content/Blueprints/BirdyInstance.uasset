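; BirdyInstance is the game instance that holds achievements and per-level high scores and handles quitting.
; Init loads both from the MainSave slot via SaveObject, and SaveGame writes them back on each death.
; UpdateScore keeps the best score per level name with a cheat flag.
; StartQuitting runs a looping timer that fades in UI_Quit until the game exits, while StopQuitting pauses it without resetting the counter.
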(event Custom|StartQuitting
  ;[1 1 1] Strange quit logic. Might cahnge later
  (bind _returnvalue (Utilities|Time|SetTimerbyEvent (delegate Custom|Exitcountdown) 0.1 true))
  (Variables|Default|SetTimerRef _returnvalue)
  (bind _returnvalue_2 (UserInterface|CreateWidget "/Game/UI/UI_Quit.UI_Quit_C"))
  (UserInterface|Viewport|AddtoViewport _returnvalue_2 0)
  (Variables|Default|SetQuitwidget _returnvalue_2))

(event Custom|StopQuitting
  ;[1 1 1] Strange quit logic. Might cahnge later
  (Utilities|Time|PauseTimerbyHandle (Variables|Default|GetTimerRef))
  (Widget|RemovefromParent (Variables|Default|GetQuitwidget)))

(event Custom|Exitcountdown
  ;[1 1 1] Strange quit logic. Might cahnge later
  (bind _output_get (Variables|Default|SetExitCounter (+ (Variables|Default|GetExitCounter) 0.05)))
  (Widget|SetRenderOpacity (Variables|/Game/UI/UI_Quit.UI_Quit_C|GetBorder_0 (Variables|Default|GetQuitwidget)) _output_get)
  (if (>= _output_get 1.0)
    (Game|QuitGame 0 "Quit" false)))

(event Custom|Recordachievements
  (params (achievement :type Stru%20Achievement%20Structure%20%28by%20ref%29))
  ;[1 1 1] Achievements
  (Utilities|Array|Add (Variables|Default|GetachievementsList) achievement))

(event Custom|UpdateScore
  (params (NewScore :type Float%20%28double-precision%29) (Is%20Cheating :type Boolean))
  ;[1 1 1] Update score
  (bind _returnvalue (Game|GetCurrentLevelName true))
  (if (> NewScore (.value (.Value (Utilities|Map|Find (Variables|Default|GetHighscoreData) _returnvalue))))
    (Utilities|Map|Add (Variables|Default|GetHighscoreData) _returnvalue (Utilities|Struct|MakeStru_Score NewScore Is%20Cheating))))

(event Custom|SaveGame
  ;[1 1 1] Save game each time we die
  (bind _returnvalue (SaveGame|CreateSaveGameObject "/Game/Blueprints/SaveObject.SaveObject_C"))
  (Variables|/Game/Blueprints/SaveObject.SaveObject_C|SetScoreList _returnvalue (Variables|Default|GetHighscoreData))
  (Variables|/Game/Blueprints/SaveObject.SaveObject_C|SetAchiList _returnvalue (Variables|Default|GetachievementsList))
  (SaveGame|SaveGametoSlot _returnvalue "MainSave"))

(event EventInit
  ;[1 1 1] Load game when game starts
  (bind _returnvalue (SaveGame|LoadGamefromSlot "MainSave"))
  (bind _assave_object (Utilities|Casting|CastToSaveObject _returnvalue))
  (Variables|Default|SetachievementsList (Variables|/Game/Blueprints/SaveObject.SaveObject_C|GetAchiList _assave_object))
  (Variables|Default|SetHighscoreData (Variables|/Game/Blueprints/SaveObject.SaveObject_C|GetScoreList _assave_object))
  (Variables|Default|SetHighscoreCheat (Variables|/Game/Blueprints/SaveObject.SaveObject_C|GetHighScoreCheat _assave_object)))