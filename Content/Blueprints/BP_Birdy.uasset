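; Player bird for a Flappy-style level, flown by the recoil of a mouse-aimed gun, with distance along X as score.
; Left click pushes the physics Body opposite the gun's up vector, while Tick aims, mirrors the mesh and checks distance and out-of-bounds achievements.
; A hit or TimeOut ragdolls the bird, saves high score and attempts to BirdyInstance, then reloads the level.
; GotAchi records new data-table achievements; Escape/P drive quitting.
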(event OnComponentHit(Body)
  (params (HitComponent :type Primitive%20Component%20Object%20Reference) (OtherActor :type Actor%20Object%20Reference) (OtherComp :type Primitive%20Component%20Object%20Reference) (NormalImpulse :type Vector :default "0, 0, 0") (Hit :type Hit%20Result%20Structure%20%28by%20ref%29))
  (bind _returnvalue (Transformation|GetActorLocation))
  (bind _skeletalmesh (Variables|Default|GetSkeletalMesh))
  (bind _body (Variables|Default|GetBody))
  (bind _returnvalue_2 (+ (.x _returnvalue) 8e+02))
  (bind _returnvalue_3 (/ _returnvalue_2 1e+01))
  (bind _returnvalue_4 (Math|Float|Max(Float) _returnvalue_3 0.0))
  ;[1 1 1] Death
  (Utilities|FlowControl|DoOnce false
    (:Completed
      (bind _asbirdy_instance (Utilities|Casting|CastToBirdyInstance (Game|GetGameInstance)))
      (if (< (Variables|/Game/Blueprints/BirdyInstance.BirdyInstance_C|GetHighScore _asbirdy_instance) _returnvalue_4)
        (Variables|/Game/Blueprints/BirdyInstance.BirdyInstance_C|SetHighScore _asbirdy_instance _returnvalue_4)
        (Variables|/Game/Blueprints/BirdyInstance.BirdyInstance_C|SetHighscoreCheat _asbirdy_instance (Variables|Default|GetIsOutside)))
      (Math|Integer|IncrementInt (Variables|/Game/Blueprints/BirdyInstance.BirdyInstance_C|GetAttempt _asbirdy_instance)
        (:%20%20
          (Effects|SpawnEmitteratLocation "/Game/StarterContent/Particles/P_Explosion.P_Explosion" (Transformation|GetActorLocation) "0, 0, 0" "3.000000,3.000000,3.000000")
          (Audio|Components|Audio|Stop (Variables|Default|GetAudio))
          (Variables|Default|SetIsDead true)
          (Collision|SetCollisionProfileName _skeletalmesh "PhysicsActor" true :!class /Script/Engine.PrimitiveComponent)
          (Physics|SetSimulatePhysics _skeletalmesh true)
          (Physics|SetSimulatePhysics _body false)
          (Collision|SetCollisionEnabled _body "NoCollision")
          (bind _returnvalue_5 (Utilities|GetDataTableRow "/Game/Blueprints/DataStuff/Data_achievement.Data_achievement" "Die")
            (:then
              (CallFunction|GotAchi _returnvalue_5)
              (Audio|PlaySound2D "/Game/StarterContent/Audio/Explosion01.Explosion01" 1.0 1.0 0.0 0 0)
              (bind _returnvalue_6 (UserInterface|CreateWidget "/Game/UI/UI_DeathScreen.UI_DeathScreen_C"))
              (UserInterface|Viewport|AddtoViewport _returnvalue_6 0)
              (Utilities|FlowControl|Delay 2.0)
              (CallFunction|Playagin))))))))

(event Custom|Playagin
  ;[1 1 1] Reset the game
  (Game|OpenLevel(byObjectReference) "/Game/Level_FlappyChallange2.Level_FlappyChallange2"))

(event Custom|TimeOut
  (bind _returnvalue (Transformation|GetActorLocation))
  (bind _skeletalmesh (Variables|Default|GetSkeletalMesh))
  (bind _body (Variables|Default|GetBody))
  (bind _returnvalue_2 (+ (.x _returnvalue) 8e+02))
  (bind _returnvalue_3 (/ _returnvalue_2 1e+01))
  (bind _returnvalue_4 (Math|Float|Max(Float) _returnvalue_3 0.0))
  ;[1 1 1] Death from time out
  (bind _returnvalue_5 (Utilities|GetDataTableRow "/Game/Blueprints/DataStuff/Data_achievement.Data_achievement" "TimeOut")
    (:then
      (CallFunction|GotAchi _returnvalue_5)
      (if (<= (.x (Transformation|GetActorLocation)) 0.0)
        (bind _returnvalue_6 (Utilities|GetDataTableRow "/Game/Blueprints/DataStuff/Data_achievement.Data_achievement" "Home")
          (:then
            (CallFunction|GotAchi _returnvalue_6))))
      ;[1 1 1] Death
      (Utilities|FlowControl|DoOnce false
        (:Completed
          (bind _asbirdy_instance (Utilities|Casting|CastToBirdyInstance (Game|GetGameInstance)))
          (if (< (Variables|/Game/Blueprints/BirdyInstance.BirdyInstance_C|GetHighScore _asbirdy_instance) _returnvalue_4)
            (Variables|/Game/Blueprints/BirdyInstance.BirdyInstance_C|SetHighScore _asbirdy_instance _returnvalue_4)
            (Variables|/Game/Blueprints/BirdyInstance.BirdyInstance_C|SetHighscoreCheat _asbirdy_instance (Variables|Default|GetIsOutside)))
          (Math|Integer|IncrementInt (Variables|/Game/Blueprints/BirdyInstance.BirdyInstance_C|GetAttempt _asbirdy_instance)
            (:%20%20
              (Effects|SpawnEmitteratLocation "/Game/StarterContent/Particles/P_Explosion.P_Explosion" (Transformation|GetActorLocation) "0, 0, 0" "3.000000,3.000000,3.000000")
              (Audio|Components|Audio|Stop (Variables|Default|GetAudio))
              (Variables|Default|SetIsDead true)
              (Collision|SetCollisionProfileName _skeletalmesh "PhysicsActor" true :!class /Script/Engine.PrimitiveComponent)
              (Physics|SetSimulatePhysics _skeletalmesh true)
              (Physics|SetSimulatePhysics _body false)
              (Collision|SetCollisionEnabled _body "NoCollision")
              (bind _returnvalue_7 (Utilities|GetDataTableRow "/Game/Blueprints/DataStuff/Data_achievement.Data_achievement" "Die")
                (:then
                  (CallFunction|GotAchi _returnvalue_7)
                  (Audio|PlaySound2D "/Game/StarterContent/Audio/Explosion01.Explosion01" 1.0 1.0 0.0 0 0)
                  (bind _returnvalue_8 (UserInterface|CreateWidget "/Game/UI/UI_DeathScreen.UI_DeathScreen_C"))
                  (UserInterface|Viewport|AddtoViewport _returnvalue_8 0)
                  (Utilities|FlowControl|Delay 2.0)
                  (CallFunction|Playagin))))))))))

(event Custom|GotAchi
  (params (MyData :type Stru%20Achievement%20Structure))
  ;[1 1 1] Got new Achievements
  (bind _asbirdy_instance (Utilities|Casting|CastToBirdyInstance (Game|GetGameInstance)))
  (if (not (Utilities|Array|ContainsItem (Variables|/Game/Blueprints/BirdyInstance.BirdyInstance_C|GetachievementsList _asbirdy_instance) MyData))
    (Default|DisplayAchievment (Variables|Default|GetUIRef) MyData)
    (Default|Recordachievements _asbirdy_instance MyData)
    (Default|AddachievementtoList (Variables|/Game/UI/UI_Score.UI_Score_C|GetUI_achievementsList (Variables|Default|GetUIRef)) MyData)))

(event EventTick
  (params (DeltaSeconds :type Float%20%28single-precision%29))
  (bind _returnvalue (Transformation|GetActorLocation))
  (bind (_returnvalue2 _facingleft) (Utilities|CalculateGun))
  (Utilities|FlowControl|Sequence
    (:then_0
      ;[1 1 1] Aim gun and freeze in place.
      (if (not (Variables|Default|GetIsDead))
        (Transformation|SetWorldRotation (Variables|Default|GetGun) (Math|Rotator|MakeRotator 0.0 _returnvalue2 0.0) false false)
        (Transformation|SetWorldScale3D (Variables|Default|GetSkeletalMesh) (Math|Vector|SelectVector "3.000000,-3.000000,3.000000" "3.000000,3.000000,3.000000" _facingleft))))
    (:then_1
      ;[1 1 1] Unused, Stop in midair
      (Utilities|FlowControl|Gate true
        (:Exit
          (Physics|SetPhysicsLinearVelocity (Variables|Default|GetBody) "0, 0, 0" false "None"))))
    (:then_2
      (if (> (/ (+ (.x (Transformation|GetActorLocation)) 8e+02) 1e+01) 9e+03)
        (Utilities|FlowControl|DoOnce false
          (:Completed
            (bind _returnvalue_2 (Utilities|GetDataTableRow "/Game/Blueprints/DataStuff/Data_achievement.Data_achievement" "Third")
              (:then
                (CallFunction|GotAchi _returnvalue_2)))))))
    (:then_3
      ;[1 1 1] See if outside
      (if (or (> (.z _returnvalue) 1.4e+03) (< (.z _returnvalue) -1e+02))
        (Utilities|FlowControl|DoOnce false
          (:Completed
            (Variables|Default|SetIsOutside true)
            (bind _returnvalue_3 (Utilities|GetDataTableRow "/Game/Blueprints/DataStuff/Data_achievement.Data_achievement" "Outside")
              (:then
                (CallFunction|GotAchi _returnvalue_3)))))))))

(event EventBeginPlay
  ;[1 1 1] Set input for the mosue
  (Variables|/Script/Engine.PlayerController|SetbShowMouseCursor (Game|GetPlayerController 0) true)
  (bind _returnvalue (UserInterface|CreateWidget "/Game/UI/UI_Score.UI_Score_C" 0 self))
  (UserInterface|Viewport|AddtoViewport _returnvalue 0)
  (Variables|Default|SetUIRef _returnvalue)
  (bind _asbirdy_instance (Utilities|Casting|CastToBirdyInstance (Game|GetGameInstance)))
  (for _array_element (Variables|/Game/Blueprints/BirdyInstance.BirdyInstance_C|GetachievementsList _asbirdy_instance)
    (Default|AddachievementtoList (Variables|/Game/UI/UI_Score.UI_Score_C|GetUI_achievementsList (Variables|Default|GetUIRef)) _array_element)))

(event Input|KeyboardEvents|SpaceBar
  (params (Key :type Key%20Structure :default "None")))

(event Input|KeyboardEvents|Escape
  (params (Key :type Key%20Structure :default "None"))
  ;[1 1 1] Exit Game logic
  (:Pressed
    (bind _asbirdy_instance (Utilities|Casting|CastToBirdyInstance (Game|GetGameInstance)))
    (Default|StartQuitting _asbirdy_instance))
  (:Released
    (bind _asbirdy_instance_2 (Utilities|Casting|CastToBirdyInstance (Game|GetGameInstance)))
    (Default|StopQuitting _asbirdy_instance_2)))

(event Input|MouseEvents|LeftMouseButton
  (params (Key :type Key%20Structure :default "None"))
  (bind _returnvalue (Transformation|GetActorLocation))
  (bind _gun (Variables|Default|GetGun))
  (bind _returnvalue_2 (Math|Vector|GetUpVector _gun))
  (bind _returnvalue_3 (* _returnvalue_2 -1.5e+05))
  (bind _returnvalue_4 (+ _returnvalue_3 _returnvalue))
  ;[1 1 1] Shooting.
  (:Pressed
    (if (not (Variables|Default|GetIsDead))
      (Niagara|SpawnSystematLocation "/Game/Materials/Particles/P_Impact_Gun.P_Impact_Gun" (Transformation|GetWorldLocation (Variables|Default|GetScene)))
      (Physics|AddForce (Variables|Default|GetBody) (Math|Vector|MakeVector (.x _returnvalue_4) 0.0 (.z _returnvalue_4)) "None" true)
      (Animation|Montage|PlayMontage (Variables|Default|GetSkeletalMesh) "/Game/FarmAnimalsPack/Chicken/Animations/ANIM_Chicken_GetHit_Montage.ANIM_Chicken_GetHit_Montage" 1.2))))

(event Input|KeyboardEvents|P
  (params (Key :type Key%20Structure :default "None"))
  ;[1 1 1] Exit Game logic
  (:Pressed
    (bind _asbirdy_instance (Utilities|Casting|CastToBirdyInstance (Game|GetGameInstance)))
    (Default|StartQuitting _asbirdy_instance))
  (:Released
    (bind _asbirdy_instance_2 (Utilities|Casting|CastToBirdyInstance (Game|GetGameInstance)))
    (Default|StopQuitting _asbirdy_instance_2)))

(fn ConstructionScript)