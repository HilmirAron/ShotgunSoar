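; Player chicken for a Flappy-style challenge, propelled by recoil from a mouse-aimed shotgun.
; Tick aims the gun and flips the mesh; clicking fires random cone line traces that destroy BP_Enemies and pushes the body opposite the shot.
; Holding Space zeroes body velocity every tick to freeze in place.
; A hit or TimeOut triggers one-time death: saves X-distance high score and attempt count to BirdyInstance, explodes, ragdolls, then reloads the level.
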(event OnComponentHit(Body)
  (params (HitComponent :type Primitive%20Component%20Object%20Reference) (OtherActor :type Actor%20Object%20Reference) (OtherComp :type Primitive%20Component%20Object%20Reference) (NormalImpulse :type Vector :default "0, 0, 0") (Hit :type Hit%20Result%20Structure%20%28by%20ref%29))
  (bind _returnvalue (Transformation|GetActorLocation))
  (bind _skeletalmesh (Variables|Default|GetSkeletalMesh))
  (bind _body (Variables|Default|GetBody))
  (bind _returnvalue_2 (+ (.x _returnvalue) 8e+02))
  (bind _returnvalue_3 (/ _returnvalue_2 1e+01))
  (bind _returnvalue_4 (Math|Float|Max(Float) _returnvalue_3 0.0))
  ;[1 1 1] Death
  (Utilities|FlowControl|DoOnce false
    (:Completed
      (bind _asbirdy_instance (Utilities|Casting|CastToBirdyInstance (Game|GetGameInstance)))
      (if (< (Variables|/Game/BirdyInstance.BirdyInstance_C|GetHighScore _asbirdy_instance) _returnvalue_4)
        (Variables|/Game/BirdyInstance.BirdyInstance_C|SetHighScore _asbirdy_instance _returnvalue_4))
      (Math|Integer|IncrementInt (Variables|/Game/BirdyInstance.BirdyInstance_C|GetAttempt _asbirdy_instance)
        (:%20%20
          (Effects|SpawnEmitteratLocation "/Game/StarterContent/Particles/P_Explosion.P_Explosion" (Transformation|GetActorLocation) "0, 0, 0" "3.000000,3.000000,3.000000")
          (Audio|Components|Audio|Stop (Variables|Default|GetAudio))
          (Variables|Default|SetIsDead true)
          (Collision|SetCollisionProfileName _skeletalmesh "PhysicsActor" true :!class /Script/Engine.PrimitiveComponent)
          (Physics|SetSimulatePhysics _skeletalmesh true)
          (Physics|SetSimulatePhysics _body false)
          (Collision|SetCollisionEnabled _body "NoCollision")
          (Audio|PlaySound2D "/Game/StarterContent/Audio/Explosion01.Explosion01" 1.0 1.0 0.0 0 0)
          (Utilities|FlowControl|Delay 2.0)
          (CallFunction|Playagin))))))

(event Custom|Playagin
  ;[1 1 1] Reset the game
  (Game|OpenLevel(byObjectReference) "/Game/Level_FlappyChallange.Level_FlappyChallange"))

(event Custom|TimeOut
  (bind _returnvalue (Transformation|GetActorLocation))
  (bind _skeletalmesh (Variables|Default|GetSkeletalMesh))
  (bind _body (Variables|Default|GetBody))
  (bind _returnvalue_2 (+ (.x _returnvalue) 8e+02))
  (bind _returnvalue_3 (/ _returnvalue_2 1e+01))
  (bind _returnvalue_4 (Math|Float|Max(Float) _returnvalue_3 0.0))
  ;[1 1 1] Death
  (Utilities|FlowControl|DoOnce false
    (:Completed
      (bind _asbirdy_instance (Utilities|Casting|CastToBirdyInstance (Game|GetGameInstance)))
      (if (< (Variables|/Game/BirdyInstance.BirdyInstance_C|GetHighScore _asbirdy_instance) _returnvalue_4)
        (Variables|/Game/BirdyInstance.BirdyInstance_C|SetHighScore _asbirdy_instance _returnvalue_4))
      (Math|Integer|IncrementInt (Variables|/Game/BirdyInstance.BirdyInstance_C|GetAttempt _asbirdy_instance)
        (:%20%20
          (Effects|SpawnEmitteratLocation "/Game/StarterContent/Particles/P_Explosion.P_Explosion" (Transformation|GetActorLocation) "0, 0, 0" "3.000000,3.000000,3.000000")
          (Audio|Components|Audio|Stop (Variables|Default|GetAudio))
          (Variables|Default|SetIsDead true)
          (Collision|SetCollisionProfileName _skeletalmesh "PhysicsActor" true :!class /Script/Engine.PrimitiveComponent)
          (Physics|SetSimulatePhysics _skeletalmesh true)
          (Physics|SetSimulatePhysics _body false)
          (Collision|SetCollisionEnabled _body "NoCollision")
          (Audio|PlaySound2D "/Game/StarterContent/Audio/Explosion01.Explosion01" 1.0 1.0 0.0 0 0)
          (Utilities|FlowControl|Delay 2.0)
          (CallFunction|Playagin))))))

(event EventTick
  (params (DeltaSeconds :type Float%20%28single-precision%29))
  (bind (_returnvalue2 _facingleft) (Utilities|CalculateGun))
  ;[1 1 1] Aim gun and freeze in place.
  (Utilities|FlowControl|Sequence
    (:then_0
      (if (not (Variables|Default|GetIsDead))
        (Transformation|SetWorldRotation (Variables|Default|GetGun) (Math|Rotator|MakeRotator 0.0 _returnvalue2 0.0) false false)
        (Transformation|SetWorldScale3D (Variables|Default|GetSkeletalMesh) (Math|Vector|SelectVector "3.000000,-3.000000,3.000000" "3.000000,3.000000,3.000000" _facingleft))))
    (:then_1
      (Utilities|FlowControl|Gate true
        (:Exit
          (Physics|SetPhysicsLinearVelocity (Variables|Default|GetBody) "0, 0, 0" false "None"))))))

(event EventBeginPlay
  ;[1 1 1] Set input for the mosue
  (Variables|/Script/Engine.PlayerController|SetbShowMouseCursor (Game|GetPlayerController 0) true)
  (bind _returnvalue (UserInterface|CreateWidget "/Game/UI_Score.UI_Score_C" 0 self))
  (UserInterface|Viewport|AddtoViewport _returnvalue 0))

(event Input|KeyboardEvents|SpaceBar
  (params (Key :type Key%20Structure :default "None"))
  ;[1 1 1] Aim gun and freeze in place.
  (:Pressed
    (Utilities|FlowControl|Gate true) ; enters at Open
  )
  (:Released
    (Utilities|FlowControl|Gate true) ; enters at Close
  ))

(event Input|MouseEvents|LeftMouseButton
  (params (Key :type Key%20Structure :default "None"))
  (bind _returnvalue (Transformation|GetActorLocation))
  (bind _scene (Variables|Default|GetScene))
  (bind _gun (Variables|Default|GetGun))
  (bind _returnvalue_2 (Math|Vector|GetUpVector _gun))
  (bind _returnvalue_3 (Transformation|GetWorldLocation _scene))
  (bind _returnvalue_4 (* _returnvalue_2 -1.5e+05))
  (bind _returnvalue_5 (+ _returnvalue_4 _returnvalue))
  ;[1 1 1] Shooting.
  (:Pressed
    (if (not (Variables|Default|GetIsDead))
      (for _index (range 0 29)
        (bind _outhit (Collision|LineTraceByChannel _returnvalue_3 (+ (* (Math|Random|RandomUnitVectorinConeinDegrees (Math|Vector|GetUpVector (Variables|Default|GetGun)) 2e+01) 4e+02) _returnvalue_3) "TraceTypeQuery1" false 0 "ForOneFrame"))
        (bind _asbp_enemies (Utilities|Casting|CastToBP_Enemies (.hitactor _outhit)))
        (Actor|DestroyActor _asbp_enemies))
      (Physics|AddForce (Variables|Default|GetBody) (Math|Vector|MakeVector (.x _returnvalue_5) 0.0 (.z _returnvalue_5)) "None" true)
      (Components|Animation|PlayAnimation (Variables|Default|GetSkeletalMesh) "/Game/FarmAnimalsPack/Chicken/Animations/ANIM_Chicken_GetHit.ANIM_Chicken_GetHit" false)
      (Utilities|FlowControl|Delay 0.4)
      (Components|Animation|PlayAnimation (Variables|Default|GetSkeletalMesh) "/Game/FarmAnimalsPack/Chicken/Animations/ANIM_Chicken_IdleLay.ANIM_Chicken_IdleLay" true))))

(fn ConstructionScript)