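; BP_PegSpawner is an actor that lays out a field of static mesh pegs.
; Its construction script runs nested loops, adding one mesh component per grid cell using configurable counts and spacing, with centering offsets and a half-spacing shift on alternate rows.
; Random position jitter and random horizontal scale vary each peg, re-rolling whenever construction reruns.
; The event graph has no active logic.
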(event EventBeginPlay)

(event Collision|EventActorBeginOverlap
  (params (OtherActor :type Actor%20Object%20Reference)))

(event EventTick
  (params (DeltaSeconds :type Float%20%28single-precision%29)))

(fn ConstructionScript
  (bind _random (Variables|Default|GetRandom))
  (bind _random_2 (Variables|Default|GetRandom))
  (bind _randomscale (Variables|Default|GetRandomScale))
  (bind _index (Variables|Default|GetIndex))
  (bind _returnvalue (Math|Random|RandomFloatinRange 8.0 _randomscale))
  (bind _returnvalue_2 (- _index 1))
  (bind _returnvalue_3 (* _returnvalue_2 0.5))
  (for _index_2 (range 0 (- (Variables|Default|GetIndex2) 1))
    (for _index_3 (range 0 (- (Variables|Default|GetIndex) 1))
      (AddComponent|AddStaticMeshComponent false (Math|Transform|MakeTransform (Math|Vector|MakeVector (+ (Utilities|Operators|Subtract (* _index_3 (Variables|Default|GetY)) (* (Variables|Default|GetY) _returnvalue_3) (select (== (Math|Integer|%(Integer) _index_2 2) 0) (/ (Variables|Default|GetY) 2.0) 0.0)) (Math|Random|RandomFloatinRange (* _random_2 -1.0) _random_2)) (+ (- (* _index_2 (Variables|Default|GetX)) (* (Variables|Default|GetX) _returnvalue_3)) (Math|Random|RandomFloatinRange (* _random -1.0) _random)) 0.0) "0, 0, 0" (Math|Vector|MakeVector _returnvalue _returnvalue 4.0))))))